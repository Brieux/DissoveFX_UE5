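; BP_Dissolve is a Blueprint that makes a static mesh disappear behind a Niagara effect after a random delay.
; BeginPlay picks a delay of up to a few seconds and sets a one-shot timer, so start times vary between instances.
; The timer event activates the Niagara component, then hides the mesh after a short pause.
; Tick is empty, and an unconnected elapsed-time check for hiding the mesh never runs.
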(event `self.ReceiveBeginPlay`
  ;[1 1 1] OUI
  (bind _output_get (set `self.DelayLaunch` (`KismetMathLibrary.RandomFloatInRange` 0.0 5.0)))
  (`KismetSystemLibrary.K2_SetTimerDelegate` (delegate `LaunchNiagara`) _output_get))

(event `LaunchNiagara`
  ;[1 1 1] OUI
  (`ActorComponent.Activate` (`self.Niagara`) true)
  (`KismetSystemLibrary.Delay` 1.0)
  (`SceneComponent.SetVisibility` (`self.StaticMesh`) false false))

(event `self.ReceiveTick`
  (params (DeltaSeconds :type "Float (single-precision)"))
  ;[1 1 1] NON
)

(fn `UserConstructionScript`)